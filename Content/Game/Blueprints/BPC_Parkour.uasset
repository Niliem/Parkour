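; Parkour component that lets the owning Character grab ledges, shimmy along them, jump between them and climb over.
; A shared sphere-trace helper sweeps forward at stepped heights, then traces down to find the ledge top for target transforms.
; Tick auto-grabs into a custom movement mode or, while climbing, updates shimmy movement and caches jump and climb targets.
; Jump and climb-over calls set location instantly; stopping briefly locks regrabbing.
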(event Custom|LockGrab
  (params (Duration :type Float%20%28single-precision%29))
  (Variables|Default|SetbLockGrab true)
  (Utilities|FlowControl|Delay Duration)
  (Variables|Default|SetbLockGrab false))

(event Custom|GrabLedge
  (bind _character (Variables|Default|GetCharacter))
  (bind _grabtransform (Variables|Default|GetGrabTransform))
  (bind _charactermovement (Variables|/Script/Engine.Character|GetCharacterMovement _character))
  (if (Variables|Default|GetbCanGrab)
    (Pawn|Components|CharacterMovement|SetMovementMode _charactermovement "MOVE_Custom" (Utilities|Enum|LiteralenumECustomMovementModes "NewEnumerator1"))
    (Components|Movement|StopMovementImmediately _charactermovement)
    (Components|MoveComponentTo (Variables|/Script/Engine.Character|GetCapsuleComponent (Variables|Default|GetCharacter)) (.location _grabtransform) (.rotation _grabtransform) true true 0.2 false)
    (Climbing|StopGrabTrace)))

(event EventTick
  (params (DeltaSeconds :type Float%20%28single-precision%29))
  (Variables|Default|GetCharacter
    (:then
      (if (Utilities|IsClimbing)
        (Utilities|FlowControl|Sequence
          (:then_0
            (Trace|TraceHorizontalMovement))
          (:then_1
            (Variables|Default|SetbCanJump false)
            (Trace|TraceVerticalJump)
            (Trace|TraceHorizontalJump))
          (:then_2
            (Trace|TraceClimb)))
        (elif (and (Variables|Default|GetbEnableGrabTrace) (not (Variables|Default|GetbLockGrab)))
          (Trace|TraceTopLedge true))))
    (:else)))

(event EventBeginPlay
  (bind _ascharacter (Utilities|Casting|CastToCharacter (Components|GetOwner)))
  (Variables|Default|SetCharacter _ascharacter))

(fn CustomTraceLedge
  (params (HorizontalOffset :type Float%20%28single-precision%29) (VerticalOffset :type Float%20%28single-precision%29) (TraceSettings :type Trace%20Settings%20Structure) (bFlipped :type Boolean) (TraceChanel :type ETraceTypeQuery%20Enum :default "TraceTypeQuery3"))
  (bind (_fowarddistance _minheight _maxheight _tracecount) (Utilities|Struct|BreakTraceSettings TraceSettings))
  (bind (_fowarddistance_2 _minheight_2 _maxheight_2 _tracecount_2 _debugmode _toptraceheight _traceradius) (Utilities|Struct|BreakTraceSettings TraceSettings))
  (bind (_fowarddistance_3 _minheight_3 _maxheight_3 _tracecount_3 _debugmode_2 _toptraceheight_2 _traceradius_2) (Utilities|Struct|BreakTraceSettings TraceSettings))
  (LocalVariables|SetL_bFindLedge false)
  (LocalVariables|SetL_Offset (+ (* (Transformation|GetActorUpVector (Variables|Default|GetCharacter)) VerticalOffset) (* (Transformation|GetActorRightVector (Variables|Default|GetCharacter)) HorizontalOffset)))
  ;[1 1 1] Forward Trace
  (bind _index (Utilities|FlowControl|ForLoopwithBreak 1 (.TraceCount (Utilities|Struct|BreakTraceSettings TraceSettings)) :!label _label)
    (:LoopBody
      (bind (_outhit _returnvalue) (Collision|SphereTraceByChannel (+ (CallFunction|GetCharacterBaseLocation 2.0) (Math|Vector|MakeVector 0.0 0.0 (* (+ (.MinHeight (Utilities|Struct|BreakTraceSettings TraceSettings)) (* (/ (- _maxheight _minheight) (Math|Conversions|ToFloat(Integer) _tracecount)) (Math|Conversions|ToFloat(Integer) _index))) (Math|Float|SelectFloat -1.0 1.0 bFlipped))) (LocalVariables|GetL_Offset)) (+ (+ (CallFunction|GetCharacterBaseLocation 2.0) (Math|Vector|MakeVector 0.0 0.0 (* (+ (.MinHeight (Utilities|Struct|BreakTraceSettings TraceSettings)) (* (/ (- _maxheight _minheight) (Math|Conversions|ToFloat(Integer) _tracecount)) (Math|Conversions|ToFloat(Integer) _index))) (Math|Float|SelectFloat -1.0 1.0 bFlipped))) (LocalVariables|GetL_Offset)) (* (Transformation|GetActorForwardVector (Variables|Default|GetCharacter)) (.FowardDistance (Utilities|Struct|BreakTraceSettings TraceSettings)))) _traceradius_2 TraceChanel false (Utilities|Array|MakeArray (Components|GetOwner)) _debugmode_2))
      (if _returnvalue
        (if (and (.bBlockingHit (Collision|BreakHitResult _outhit)) (not (.bInitialOverlap (Collision|BreakHitResult _outhit))))
          (LocalVariables|SetL_ImpactLocation (.ImpactPoint (Collision|BreakHitResult _outhit)))
          (LocalVariables|SetL_ImpactNormal (.ImpactNormal (Collision|BreakHitResult _outhit)))
          (LocalVariables|SetL_bFindLedge true))
        (elif (LocalVariables|GetL_bFindLedge)
          (goto _label Break))))
    (:Completed
      ;[1 1 1] Downward Trace
      (if (LocalVariables|GetL_bFindLedge)
        (bind (_outhit_2 _returnvalue_2) (Collision|SphereTraceByChannel (+ (+ (Math|Vector|MakeVector (.x (LocalVariables|GetL_ImpactLocation)) (.y (LocalVariables|GetL_ImpactLocation)) (.z (LocalVariables|GetL_ImpactLocation))) (* (LocalVariables|GetL_ImpactNormal) -15.0)) (Math|Vector|MakeVector 0.0 0.0 (.TopTraceHeight (Utilities|Struct|BreakTraceSettings TraceSettings)))) (+ (Math|Vector|MakeVector (.x (LocalVariables|GetL_ImpactLocation)) (.y (LocalVariables|GetL_ImpactLocation)) (.z (LocalVariables|GetL_ImpactLocation))) (* (LocalVariables|GetL_ImpactNormal) -15.0)) _traceradius TraceChanel false (Utilities|Array|MakeArray (Components|GetOwner)) _debugmode true "(R=0.000000,G=0.266369,B=1.000000,A=1.000000)" "(R=0.868490,G=0.000000,B=1.000000,A=1.000000)"))
        (if _returnvalue_2
          (LocalVariables|SetL_DownTraceLocation (Math|Vector|MakeVector (.x (.Location (Collision|BreakHitResult _outhit_2))) (.y (.Location (Collision|BreakHitResult _outhit_2))) (.z (.ImpactPoint (Collision|BreakHitResult _outhit_2)))))
          (return true (LocalVariables|GetL_ImpactLocation) (LocalVariables|GetL_ImpactNormal) (LocalVariables|GetL_DownTraceLocation))
          (else
            (return false "0, 0, 0" "0, 0, 0" "0, 0, 0")))
        (else
          (return false "0, 0, 0" "0, 0, 0" "0, 0, 0"))))))

(fn TraceTopLedge
  (params (bAutoGrab :type Boolean))
  (if (Variables|Default|GetbEnableGrabTrace)
    (bind (_bfindledge _impactlocation _impactnormal _downtracelocation) (Trace|CustomTraceLedge 0.0 0.0 (Variables|Trace|GetGrabLedgeSettings) false "TraceTypeQuery3"))
    (if _bfindledge
      (LocalVariables|SetL_ImpactLocation _impactlocation)
      (LocalVariables|SetL_ImpactNormal _impactnormal)
      (LocalVariables|SetL_DownTraceLocation _downtracelocation)
      ;[1 1 1] Grab
      (CallFunction|SetCanGrab (and (Math|Float|InRange(Float) (- (.Z (Math|Vector|BreakVector (LocalVariables|GetL_DownTraceLocation))) (.z (Transformation|GetSocketLocation (Variables|/Script/Engine.Character|GetMesh (Variables|Default|GetCharacter)) (Variables|Settings|GetSocket)))) 0.0 (Variables|Settings|GetGrabMaxDistance)) (not (Utilities|IsClimbing))))
      (if (and (Math|Float|InRange(Float) (- (.Z (Math|Vector|BreakVector (LocalVariables|GetL_DownTraceLocation))) (.z (Transformation|GetSocketLocation (Variables|/Script/Engine.Character|GetMesh (Variables|Default|GetCharacter)) (Variables|Settings|GetSocket)))) 0.0 (Variables|Settings|GetGrabMaxDistance)) (not (Utilities|IsClimbing)))
        (Variables|Default|SetGrabTransform (CallFunction|CalcTargetTransform (LocalVariables|GetL_ImpactLocation) (LocalVariables|GetL_ImpactNormal) (LocalVariables|GetL_DownTraceLocation)))
        (if bAutoGrab
          (CallFunction|GrabLedge))))
    (else
      (CallFunction|SetCanGrab false))))

(fn GetCharacterBaseLocation
  (params (ZOffset :type Float%20%28single-precision%29))
  (bind _character (Variables|Default|GetCharacter))
  (return (- (Transformation|GetActorLocation _character) (* (Transformation|GetActorUpVector _character) (+ (Components|Capsule|GetScaledCapsuleHalfHeight (Variables|/Script/Engine.Character|GetCapsuleComponent _character)) ZOffset)))))

(fn AddHorizontalMovement
  (params (Input :type Float%20%28single-precision%29))
  (Variables|Default|SetMovementVector (Math|Vector2D|MakeVector2D Input (.y (Variables|Default|GetMovementVector)))))

(fn AddVerticalMovement
  (params (Input :type Float%20%28single-precision%29))
  (Variables|Default|SetMovementVector (Math|Vector2D|MakeVector2D (.x (Variables|Default|GetMovementVector)) Input)))

(fn CanGrab
  (return (Variables|Default|GetbCanGrab)))

(fn SetCanGrab
  (params (bCan :type Boolean))
  (if (Math|Boolean|NotEqual(Boolean) bCan (CallFunction|CanGrab))
    (bind _output_get (Variables|Default|SetbCanGrab bCan))
    (Default|CallOnCanGrabChange _output_get)))

(fn StartGrabTrace
  (Variables|Default|SetbEnableGrabTrace true))

(fn StopGrabTrace
  (Variables|Default|SetbEnableGrabTrace false))

(fn StopClimbing
  (bind _character (Variables|Default|GetCharacter)
    (:then
      (Pawn|Components|CharacterMovement|SetMovementMode (Variables|/Script/Engine.Character|GetCharacterMovement _character) "MOVE_Walking" 0)
      (Variables|Default|SetbEnableGrabTrace false)
      (CallFunction|LockGrab 0.3))
    (:else)))

(fn TraceHorizontalMovement
  (bind _movementvector (Variables|Default|GetMovementVector))
  (if (> (Math|Float|Absolute(Float) (.x _movementvector)) 0.0)
    (bind (_bfindledge _impactlocation _impactnormal _downtracelocation) (Trace|CustomTraceLedge (* (.x _movementvector) 3e+01) 0.0 (Variables|Trace|GetHorizontalMovementSettings) false "TraceTypeQuery3"))
    (bind _output_get (Variables|Default|SetbCanMove _bfindledge))
    (if _output_get
      (Transformation|SetActorLocationAndRotation (Variables|Default|GetCharacter) (Math|Interpolation|VInterpTo (Transformation|GetActorLocation (Variables|Default|GetCharacter)) (.location (CallFunction|CalcTargetTransform _impactlocation _impactnormal _downtracelocation)) (Utilities|Time|GetWorldDeltaSeconds) (Variables|Settings|GetLeftRightSpeed)) (Class|KismetMathLibrary|RInterptoConstant (Transformation|GetActorRotation (Variables|Default|GetCharacter)) (.rotation (CallFunction|CalcTargetTransform _impactlocation _impactnormal _downtracelocation)) (Utilities|Time|GetWorldDeltaSeconds) 0.0)))
    (else
      (Variables|Default|SetbCanMove false))))

(fn CalcTargetTransform
  (params (ImpactLocation :type Vector) (ImpactNormal :type Vector) (DownTraceLocation :type Vector))
  (bind _grabdistanceoffset (Variables|Settings|GetGrabDistanceOffset))
  (bind _returnvalue (* ImpactNormal _grabdistanceoffset))
  (bind _returnvalue_2 (+ _returnvalue ImpactLocation))
  (return (Math|Transform|MakeTransform (Math|Vector|MakeVector (.x _returnvalue_2) (.y _returnvalue_2) (- (.Z (Math|Vector|BreakVector DownTraceLocation)) (Variables|Settings|GetGrabHeight))) (Math|Rotator|MakeRotfromX (* ImpactNormal -1.0)))))

(fn TraceHorizontalJump
  (if (> (Math|Float|Absolute(Float) (.x (Variables|Default|GetMovementVector))) 0.0)
    (bind _index (Utilities|FlowControl|ForLoopwithBreak 2 5 :!label _label)
      (:LoopBody
        (bind (_bfindledge _impactlocation _impactnormal _downtracelocation) (Trace|CustomTraceLedge (* _index (* (.x (Variables|Default|GetMovementVector)) 5e+01)) 0.0 (Variables|Trace|GetHorizontalJumpSettings) false "TraceTypeQuery3"))
        (bind _output_get (Variables|Default|SetbCanJump _bfindledge))
        (if _output_get
          (Variables|Default|SetJumpLocation (.location (CallFunction|CalcTargetTransform _impactlocation _impactnormal _downtracelocation)))
          (goto _label Break))))))

(fn TryJumptoNextLedge
  (if (Variables|Default|GetbCanJump)
    (Transformation|SetActorLocation (Variables|Default|GetCharacter) (Variables|Default|GetJumpLocation) false false)
    (Climbing|StartGrabTrace)
    (return true)
    (else
      (return false))))

(fn TraceVerticalJump
  (bind _movementvector (Variables|Default|GetMovementVector))
  (bind _returnvalue (> (.y _movementvector) 0.0))
  (if (> (Math|Float|Absolute(Float) (.y (Variables|Default|GetMovementVector))) 0.0)
    (bind _array_element (Utilities|Array|ForEachLoopwithBreak (Utilities|Array|MakeArray 0 1 -1) :!label _label)
      (:LoopBody
        (bind (_bfindledge _impactlocation _impactnormal _downtracelocation) (Trace|CustomTraceLedge (* _array_element (* (.y (Variables|Default|GetMovementVector)) 5e+01)) 0.0 (select _returnvalue (Variables|Trace|GetVerticalJumpSettings) (Variables|Trace|GetVerticalJumpDownSettings)) (not _returnvalue) "TraceTypeQuery3"))
        (bind _output_get (Variables|Default|SetbCanJump _bfindledge))
        (if _output_get
          (Variables|Default|SetJumpLocation (.location (CallFunction|CalcTargetTransform _impactlocation _impactnormal _downtracelocation)))
          (goto _label Break))))))

(fn TraceClimb
  (bind _character (Variables|Default|GetCharacter))
  (bind _character_2 (Variables|Default|GetCharacter))
  (bind _returnvalue (Transformation|GetActorUpVector _character_2))
  (bind _capsulecomponent (Variables|/Script/Engine.Character|GetCapsuleComponent _character_2))
  (bind _returnvalue_2 (Components|Capsule|GetScaledCapsuleRadius _capsulecomponent))
  (bind (_bfindledge _impactlocation _impactnormal _downtracelocation) (Trace|CustomTraceLedge 0.0 0.0 (Variables|Trace|GetClimbSettings) false "TraceTypeQuery1"))
  (if _bfindledge
    (bind _returnvalue_3 (Collision|SphereTraceByChannel (+ _downtracelocation (* _returnvalue (+ _returnvalue_2 2.0))) (+ (+ _downtracelocation (* _returnvalue (+ _returnvalue_2 2.0))) (* _returnvalue (Components|Capsule|GetScaledCapsuleHalfHeight _capsulecomponent))) _returnvalue_2 "TraceTypeQuery1" false 0 "ForOneFrame"))
    (Variables|Default|SetbCanClimb (not _returnvalue_3))
    (Variables|Default|SetClimbLocation (+ _downtracelocation (* (Transformation|GetActorUpVector _character) (Components|Capsule|GetScaledCapsuleHalfHeight (Variables|/Script/Engine.Character|GetCapsuleComponent _character)))))
    (else
      (Variables|Default|SetbCanClimb false))))

(fn TryClimbOver
  (if (Variables|Default|GetbCanClimb)
    (Transformation|SetActorLocation (Variables|Default|GetCharacter) (Variables|Default|GetClimbLocation) false false)
    (Climbing|StopClimbing)))